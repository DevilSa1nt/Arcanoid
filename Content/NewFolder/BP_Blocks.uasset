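; Brick grid for a ball-and-blocks game, built from static mesh components in the construction script.
; On BeginPlay it registers with the player controller and replaces each mesh with a spawned MyDistObj actor, blanking the original.
; Restart rebuilds the grid, destroys those actors and repeats the swap.
; Its Hit handler makes BP_Ball hits switch a component's material, then destroy it with particles and a chance of BP_Bonus.
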(event `Restart`
  (`self.NewFunction`)
  (for _array_element (`self.Objs`)
    (if (`KismetSystemLibrary.IsValid` _array_element)
      (`self.K2_DestroyActor` _array_element)))
  (bind _asmy_my_player_controller (cast `/Game/NewFolder/MyMyPlayerController` (`GameplayStatics.GetPlayerController` 0) :!label _label))
  (set `/Game/NewFolder/MyMyPlayerController.Blocks` self _asmy_my_player_controller)
  (for _array_element_2 (`self.Meshes`)
    (bind _returnvalue (`|SpawnActorFromClass` "/Game/NewFolder/MyDistObj.MyDistObj_C" (`KismetMathLibrary.MakeTransform` (`SceneComponent.K2_GetComponentLocation` _array_element_2) (struct) (`SceneComponent.K2_GetComponentScale` _array_element_2)) "AlwaysSpawn" "MultiplyWithRoot" null (`StaticMeshComponent.StaticMesh` _array_element_2) null))
    (`KismetArrayLibrary.Array_Add` (`self.Objs`) _returnvalue)
    (`StaticMeshComponent.SetStaticMesh` _array_element_2 null)))

(event `self.ReceiveBeginPlay`
  (goto _label))

(event `self.ReceiveHit`
  (params (MyComp :type "PrimitiveComponent Object Reference") (Other :type "Actor Object Reference") (OtherComp :type "PrimitiveComponent Object Reference") (bSelfMoved :type Boolean) (HitLocation :type "Vector Structure") (HitNormal :type "Vector Structure") (NormalImpulse :type "Vector Structure") (Hit :type "HitResult Structure (by ref)"))
  (bind _returnvalue (`PrimitiveComponent.GetMaterial` MyComp 0))
  (cast `/Game/NewFolder/BP_Ball` Other)
  (if (== _returnvalue (`self.M1`))
    (`PrimitiveComponent.SetMaterial` MyComp 0 (`self.M2`))
    (elif (== _returnvalue (`self.M2`))
      (`self.SpawnBonus` MyComp)
      (bind _returnvalue_2 (`AddComponent|NODE_AddParticleSystemComponent-0` :`RelativeTransform` (`KismetMathLibrary.MakeTransform` (`SceneComponent.RelativeLocation` MyComp))))
      (`ActorComponent.K2_DestroyComponent` MyComp)
      (`KismetSystemLibrary.Delay` 3.0)
      (`ActorComponent.K2_DestroyComponent` _returnvalue_2))))

(fn `NewFunction`
  (bind _padding (`self.Padding`))
  (bind _scale (`self.Scale`))
  (for _index (range (+ (`self.X_Num`) 1))
    (for _index_2 (range (+ (`self.Y_Num`) 1))
      (bind _returnvalue (`AddComponent|NODE_AddStaticMeshComponent-0` :`RelativeTransform` (`KismetMathLibrary.MakeTransform` (`KismetMathLibrary.MakeVector` (`KismetMathLibrary.Conv_IntToDouble` (* _index _padding)) (`KismetMathLibrary.Conv_IntToDouble` (* _index_2 _padding))) (struct) (`KismetMathLibrary.MakeVector` _scale _scale _scale))))
      (`KismetArrayLibrary.Array_Add` (`self.Meshes`) _returnvalue)
      (`StaticMeshComponent.SetStaticMesh` _returnvalue (`self.StaticMesh`))
      (`PrimitiveComponent.SetMaterial` _returnvalue 0 (`self.M1`)))))

(fn `SpawnBonus`
  (params (self2 :type "SceneComponent Object Reference"))
  (if (`KismetMathLibrary.RandomBoolWithWeight` (`self.BonusChance`))
    (`|SpawnActorFromClass` "/Game/NewFolder/BP_Bonus.BP_Bonus_C" (`KismetMathLibrary.MakeTransform` (`SceneComponent.K2_GetComponentLocation` self2)) "AlwaysSpawn" "MultiplyWithRoot" null null null)))

(fn `UserConstructionScript`
  (`self.NewFunction`))