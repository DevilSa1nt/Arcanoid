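; BP_Pawn is the player paddle in an Arkanoid-style game, moving sideways with sweep and rotating within a limited yaw range.
; It spawns and counts balls; when the last dies, it either updates lives and respawns or shows game over through the controller's widget.
; Overlapped BP_Bonus pickups add balls or temporarily change paddle speed.
; BeginPlay starts the game mode and saves the base transform, which Restart restores while resetting game state.
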(event `self.ReceiveActorBeginOverlap`
  (params (OtherActor :type "Actor Object Reference"))
  (bind _asbp_bonus (cast `/Game/NewFolder/BP_Bonus` OtherActor))
  (bind _output_get (set `self.As BP Bonus` _asbp_bonus))
  (set `self.SpeedMult` (`/Game/NewFolder/BP_Bonus.SpeedKoeff` _output_get))
  (bind _output_get_2 (set `self.AddBall` (`/Game/NewFolder/BP_Bonus.AddBall` _output_get)))
  (if (> _output_get_2 0)
    (for _ (range (`self.AddBall`))
      (`self.SpawnBall`))
    (`self.K2_DestroyActor` (`self.As BP Bonus`))
    (elif (> (`self.SpeedMult`) 1.0)
      (`self.K2_DestroyActor` (`self.As BP Bonus`))
      (`KismetSystemLibrary.Delay` (`self.SpeedMultTime`))
      (set `self.SpeedMult` 1.0))))

(event `OnDeadReaction`
  (bind _output_get (set `self.CountOfBalls` (- (`self.CountOfBalls`) 1)))
  (if (== _output_get 0)
    (bind _result (`/Engine/EditorBlueprintResources/StandardMacros.DecrementInt` (`self.Lives`))
      (:`  `
        (if (== _result 0)
          (`/Game/NewFolder/NewWidgetBlueprint.GameOver` (`self.Widget`))
          (else
            (`/Game/NewFolder/NewWidgetBlueprint.ChangeLives` (stale `self.ReceiveBeginPlay` _output_get) (`self.Lives`) :!label _label)
            (`self.SpawnBall`)))))))

(event `self.ReceiveBeginPlay`
  (bind _asmy_arcanoid_game_mode_base (cast `/Game/NewFolder/MyArcanoidGameModeBase` (`GameplayStatics.GetGameMode`)))
  (`/Game/NewFolder/MyArcanoidGameModeBase.Start` _asmy_arcanoid_game_mode_base)
  (`self.SetBaseTransform` true)
  (bind _asmy_my_player_controller (cast `/Game/NewFolder/MyMyPlayerController` (`GameplayStatics.GetPlayerController` 0) :!label _label_2))
  (bind _output_get (set `self.Widget` (`/Game/NewFolder/MyMyPlayerController.Widget` _asmy_my_player_controller)))
  (set `self.Lives` 1)
  (goto _label))

(event `Restart`
  (`self.SetBaseTransform` false)
  (set `self.Speed` 10.0)
  (`KismetArrayLibrary.Array_Clear` (`self.PlayingBall`))
  (set `self.CountOfBalls` 0)
  (goto _label_2))

(event `InputAxis|MoveRight`
  (params (AxisValue :type "Float (single-precision)"))
  (`self.K2_AddActorWorldOffset` (`KismetMathLibrary.MakeVector` (* (/ AxisValue (`KismetMathLibrary.Abs` AxisValue)) (`self.Speed`) (`self.SpeedMult`))) true))

(event `InputAxis|Rotate`
  (params (AxisValue :type "Float (single-precision)"))
  (bind (_returnvalue_roll _returnvalue_pitch _returnvalue_yaw) (`KismetMathLibrary.BreakRotator` (`self.K2_GetActorRotation`)))
  (bind _returnvalue (+ AxisValue _returnvalue_yaw))
  (if (and (< _returnvalue 45.0) (> _returnvalue -45.0))
    (`self.K2_SetActorRotation` (`KismetMathLibrary.MakeRotator` 0.0 0.0 _returnvalue))))

(fn `SetBaseTransform`
  (params (`Set/Get` :type Boolean))
  (if `Set/Get`
    (set `self.BaseTransform` (`SceneComponent.K2_GetComponentToWorld` (`self.Cube`)))
    (else
      (`SceneComponent.K2_SetWorldTransform` (`self.Cube`) (`self.BaseTransform`) false true))))

(fn `SpawnBall`
  (bind _returnvalue_location (`KismetMathLibrary.BreakTransform` (`SceneComponent.K2_GetComponentToWorld` (`self.Capsule`))))
  (bind _returnvalue (`|SpawnActorFromClass` "/Game/NewFolder/BP_Ball.BP_Ball_C" (`KismetMathLibrary.MakeTransform` _returnvalue_location) "AlwaysSpawn" "MultiplyWithRoot" null null))
  (`KismetArrayLibrary.Array_Add` (`self.PlayingBall`) _returnvalue)
  (add `/Game/NewFolder/BP_Ball.OnDead` _returnvalue (`|CreateDelegate` :!event `OnDeadReaction`))
  (set `self.CountOfBalls` (+ 1 (`self.CountOfBalls`))))

(fn `UserConstructionScript`)