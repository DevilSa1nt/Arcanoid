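; BP_Bonus is a moving pickup that carries either a speed or an extra-ball bonus.
; On BeginPlay it compares its Material with those on its MyDistObj owner, setting SpeedKoeff or AddBall and applying the matching material to its Cube.
; Tick sweeps the Cube along Direction at Speed, scaled by delta time.
; The actor destroys itself on overlapping a KillZVolume; applying the bonus happens outside these graphs.
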(event `self.ReceiveActorBeginOverlap`
  (params (OtherActor :type "Actor Object Reference"))
  (cast `KillZVolume` OtherActor)
  (`self.K2_DestroyActor`))

(event `self.ReceiveTick`
  (params (DeltaSeconds :type "Float (single-precision)"))
  (`SceneComponent.K2_AddWorldOffset` (`self.Cube`) (* DeltaSeconds (* (`self.Direction`) (`self.Speed`))) true false))

(event `self.ReceiveBeginPlay`
  (bind _asmy_dist_obj (cast `/Game/NewFolder/MyDistObj` (`self.GetOwner`)))
  (if (== (`self.Material`) (`/Game/NewFolder/MyDistObj.SpeedBonusMaterial` _asmy_dist_obj))
    (set `self.SpeedKoeff` 2.0)
    (`PrimitiveComponent.SetMaterial` (`self.Cube`) 0 (`self.Material`) :!label _label)
    (elif (== (`self.Material`) (`/Game/NewFolder/MyDistObj.AddBallMaterial` _asmy_dist_obj))
      (set `self.AddBall` 1)
      (goto _label))))

(fn `UserConstructionScript`)